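; BP_OperacionesMatematicas is a class-exercise Blueprint that demonstrates basic arithmetic through custom functions.
; It defines functions to add, subtract, divide and multiply two numbers.
; On BeginPlay it subtracts Vida from VidaAdicional and prints the result on screen.
; The addition, division and multiplication functions are never called, and division has no zero check.
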(event EventBeginPlay
  (bind _resultado (CallFunction|RestarDosNumeros (Variables|Props|GetvidaAdicional) (Variables|Props|Getvida)))
  (Development|PrintString (Utilities|String|ToString(Integer) _resultado) true true "(R=0.000000,G=0.660000,B=1.000000,A=1.000000)" 4e+01))

(event Collision|EventActorBeginOverlap
  (params (OtherActor :type Actor%20Object%20Reference)))

(event EventTick
  (params (DeltaSeconds :type Float%20%28single-precision%29)))

(fn ConstructionScript)

(fn SumarDosNumeros
  (params (num1 :type Integer) (num2 :type Integer))
  (return (+ num1 num2)))

(fn RestarDosNumeros
  (params (num1 :type Integer) (num2 :type Integer))
  (return (- num1 num2)))

(fn DividirDosNumeros
  (params (num1 :type Integer) (num2 :type Integer))
  (return (/ num1 num2)))

(fn MultiplicarDosNumeros
  (params (Num1 :type Integer) (Num2 :type Integer))
  (return (* Num1 Num2)))