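; BP_ActorA is a simple actor that moves and spins continuously, driven by its Velocidad and Velrotacion variables.
; On BeginPlay it prints its Nombre, speed and rotation values as a long-lived debug message.
; Each Tick adds the rotation and offset in local space, without sweep or delta-time scaling, so motion depends on frame rate and follows the actor's changing orientation.
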(event EventBeginPlay
  (Development|PrintString (Utilities|String|Append "Nombre: 
" (Variables|Propiedades|Getnombre) " 
Velocidad: 
" (Utilities|String|ToString(Vector) (Variables|Propiedades|Getvelocidad)) " 
Velrotacion: 
" (Utilities|String|ToString(Rotator) (Variables|Propiedades|Getvelrotacion))) true true "(R=0.000000,G=0.660000,B=1.000000,A=1.000000)" 2e+01))

(event Collision|EventActorBeginOverlap
  (params (OtherActor :type Actor%20Object%20Reference)))

(event EventTick
  (params (DeltaSeconds :type Float%20%28single-precision%29))
  (Transformation|AddActorLocalRotation (Variables|Propiedades|Getvelrotacion) false false)
  (Transformation|AddActorLocalOffset (Variables|Propiedades|Getvelocidad) false false))

(fn ConstructionScript)