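; BP_ActorC is an actor that rotates and moves continuously, driven by its Nombre, Velocidad and Velrotacion variables.
; On BeginPlay it prints all three values to the screen.
; Each Tick adds Velrotacion as local rotation, then applies Velocidad as both a local and a world offset without sweep.
; Movement and rotation are per frame, with no delta-time scaling.
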(event EventBeginPlay
  (Development|PrintString (Utilities|String|Append "Nombre: 
" (Variables|propiedades|Getnombre) " 
Velocidad: 
" (Utilities|String|ToString(Vector) (Variables|propiedades|Getvelocidad)) " 
Velrotacion: 
" (Utilities|String|ToString(Rotator) (Variables|propiedades|Getvelrotacion))) true true "(R=0.000000,G=0.660000,B=1.000000,A=1.000000)" 2e+01))

(event Collision|EventActorBeginOverlap
  (params (OtherActor :type Actor%20Object%20Reference)))

(event EventTick
  (params (DeltaSeconds :type Float%20%28single-precision%29))
  (bind _velocidad (Variables|propiedades|Getvelocidad))
  (Transformation|AddActorLocalRotation (Variables|propiedades|Getvelrotacion) false false)
  (Transformation|AddActorLocalOffset _velocidad false false)
  (Transformation|AddActorWorldOffset _velocidad))

(fn ConstructionScript)