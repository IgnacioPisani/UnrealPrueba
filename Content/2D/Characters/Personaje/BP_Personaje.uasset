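; BP_Personaje is the player character for a 2D side-on game, with horizontal movement, jumping, coins and health.
; BeginPlay adds the Enhanced Input mapping context that drives movement along world X and jumping.
; The sign of the X acceleration flips control rotation between 0 and 180 yaw to face the travel direction.
; ObtenerMonedas and Curar update coins (Monedas) and health (Vida), printing the totals on screen.
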(event Input|EnhancedActionEvents|EnhancedInputActionIA_Movimiento
  (params (ActionValue :type Float%20%28double-precision%29) (ElapsedSeconds :type Float%20%28double-precision%29) (TriggeredSeconds :type Float%20%28double-precision%29) (InputAction :type Input%20Action%20Object%20Reference :default "/Game/Inputs/InputAction/IA_Movimiento.IA_Movimiento"))
  (bind _returnvalue (Pawn|GetController))
  (Pawn|Input|AddMovementInput "1.000000,0.000000,0.000000" ActionValue false)
  (Math|Float|CompareFloat (.x (Pawn|Components|CharacterMovement|GetCurrentAcceleration (Variables|Character|GetCharacterMovement))) 0.0
    (:>
      (Pawn|SetControlRotation _returnvalue (Math|Rotator|MakeRotator 0.0 0.0 0.0)))
    (:<
      (Pawn|SetControlRotation _returnvalue (Math|Rotator|MakeRotator 0.0 0.0 1.8e+02)))))

(event Input|EnhancedActionEvents|EnhancedInputActionIA_Salto
  (params (ActionValue :type Boolean) (ElapsedSeconds :type Float%20%28double-precision%29) (TriggeredSeconds :type Float%20%28double-precision%29) (InputAction :type Input%20Action%20Object%20Reference :default "/Game/Inputs/InputAction/IA_Salto.IA_Salto"))
  (:Started
    (Character|Jump))
  (:Completed
    (Character|StopJumping)))

(event EventBeginPlay
  (bind _asplayer_controller (Utilities|Casting|CastToPlayerController (Pawn|GetController)))
  (Input|AddMappingContext (PlayerController|LocalPlayerSubsystems|GetEnhancedInputLocalPlayerSubsystem _asplayer_controller) "/Game/Inputs/MappingContext/IMC_PersonajeInputs.IMC_PersonajeInputs" 0 "(bIgnoreAllPressedKeysUntilRelease=True,bForceImmediately=False,bNotifyUserSettings=False)"))

(event EventObtenerMonedas
  (params (Monedas :type Integer))
  (bind _output_get (Variables|Mochila|SetMonedas (+ Monedas (Variables|Mochila|GetMonedas))))
  (Development|PrintString (Utilities|String|ToString(Integer) _output_get) true true "(R=0.000000,G=0.660000,B=1.000000,A=1.000000)" 6.0))

(event EventCurar
  (params (RegenSalud :type Float%20%28double-precision%29))
  (bind _output_get (Variables|Propiedades|SetVida (+ RegenSalud (Variables|Propiedades|GetVida))))
  (Development|PrintString (Utilities|String|ToString(Float) _output_get) true true "(R=0.085229,G=1.000000,B=0.086275,A=1.000000)" 6.0))

(fn ConstructionScript)